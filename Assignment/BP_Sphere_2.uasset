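; BP_Sphere_2 is a grabbable sphere that changes its look when picked up.
; On grab, it applies a random material from MaterialArry, skipping the first entry, and passes Collapse01 to SphereCollision as a link sound message.
; The construction script stores a dynamic material instance that no graph here uses.
; MaterialArryLoop is never called here, and its modulo-by-1 index always resolves to zero.
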(event OnGrabbed(GrabComponent)
  (CallFunction|MaterialArryLoopRandom)
  (Class|AudioLinkBlueprintInterface|SetLinkSound(Message) (Variables|Default|GetSphereCollision) "/Game/StarterContent/Audio/Collapse01.Collapse01"))

(event EventBeginPlay)

(event Collision|EventActorBeginOverlap
  (params (OtherActor :type Actor%20Object%20Reference)))

(event EventTick
  (params (DeltaSeconds :type Float%20%28single-precision%29)))

(fn ConstructionScript
  (bind _returnvalue (Rendering|Material|CreateDynamicMaterialInstance (Variables|Default|GetSM_Sphere2) 0 0 "None" :!class /Script/Engine.PrimitiveComponent))
  (Variables|Default|SetDynamicMaterial _returnvalue))

(fn MaterialArryLoop
  (bind _materialarry (Variables|Default|GetMaterialArry))
  (bind _output_get (Variables|Default|SetGetCurrentValue (Math|Integer|%(Integer) (Math|Integer|%(Integer) (Variables|Default|GetGetCurrentValue) 1) (Utilities|Array|Length _materialarry))))
  (Rendering|Material|SetMaterial (Variables|Default|GetSM_Sphere2) 0 (Utilities|Array|Get(acopy) _materialarry _output_get)))

(fn MaterialArryLoopRandom
  (bind _materialarry (Variables|Default|GetMaterialArry))
  (Rendering|Material|SetMaterial (Variables|Default|GetSM_Sphere2) 0 (Utilities|Array|Get(acopy) _materialarry (Math|Random|RandomIntegerinRange 1 (- (Utilities|Array|Length _materialarry) 1)))))