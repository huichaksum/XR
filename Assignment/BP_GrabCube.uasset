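; BP_GrabCube is a grabbable cube actor that switches to the next material each time it is grabbed.
; GrabComponent's OnGrabbed event calls MaterialArrayLoop, which advances a wrapping index through MaterialArray and applies that material to SMGrabCube.
; MaterialArrayRandom offers a random pick that skips the first entry but is not called here.
; The construction script stores a dynamic material instance that nothing here uses.
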(event OnGrabbed(GrabComponent)
  (CallFunction|MaterialArrayLoop))

(event EventBeginPlay)

(event Collision|EventActorBeginOverlap
  (params (OtherActor :type Actor%20Object%20Reference)))

(event EventTick
  (params (DeltaSeconds :type Float%20%28single-precision%29)))

(fn ConstructionScript
  (bind _returnvalue (Rendering|Material|CreateDynamicMaterialInstance (Variables|Default|GetSM_GrabCube) 0 0 "None" :!class /Script/Engine.PrimitiveComponent))
  (Variables|Default|SetDynamicMaterial _returnvalue))

(fn MaterialArrayLoop
  (bind _materialarray (Variables|Default|GetMaterialArray))
  (bind _output_get (Variables|Default|SetCurrentValue (Math|Integer|%(Integer) (+ (Variables|Default|GetCurrentValue) 1) (Utilities|Array|Length _materialarray))))
  (Rendering|Material|SetMaterial (Variables|Default|GetSM_GrabCube) 0 (Utilities|Array|Get(acopy) _materialarray _output_get)))

(fn MaterialArrayRandom
  (bind _materialarray (Variables|Default|GetMaterialArray))
  (Rendering|Material|SetMaterial (Variables|Default|GetSM_GrabCube) 0 (Utilities|Array|Get(acopy) _materialarray (Math|Random|RandomIntegerinRange 1 (- (Utilities|Array|Length _materialarray) 1)))))